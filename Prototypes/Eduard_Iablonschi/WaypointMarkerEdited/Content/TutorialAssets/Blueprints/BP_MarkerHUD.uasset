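; HUD Blueprint that draws a marker and a distance label in meters for each objective stored through SetObjective.
; DrawHUD uses dot products and screen projection to draw objectives ahead and within vertical screen bounds above their projected position.
; Objectives behind the player or outside those bounds get a rotated material on a circle around screen center, with angles derived from arccosine and height clamped to the viewport.
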(event EventBeginPlay)

(event Collision|EventActorBeginOverlap
  (params (OtherActor :type Actor%20Object%20Reference)))

(event EventTick
  (params (DeltaSeconds :type Float%20%28single-precision%29)))

(event EventSetObjective
  (params (Objective :type Array%20of%20Actor%20Object%20References))
  (Variables|Default|SetCurrent%20Objective Objective))

(event EventDrawHUD
  (params (SizeX :type Integer) (SizeY :type Integer))
  (bind _returnvalue (Viewport|GetViewportSize))
  (bind _returnvalue_2 (Viewport|GetViewportSize))
  (bind _returnvalue_3 (Viewport|GetViewportSize))
  (bind _returnvalue_4 (Viewport|GetViewportSize))
  (bind _returnvalue_5 (/ _returnvalue 2.0))
  (bind _returnvalue_6 (/ _returnvalue_2 2.0))
  (bind _returnvalue_7 (/ _returnvalue_3 2.0))
  (bind _returnvalue_8 (/ _returnvalue_4 2.0))
  (for _array_element (Variables|Default|GetCurrent%20Objective)
    (Variables|Default|SetObjective%20Text (Utilities|String|Append "Objective" (Utilities|String|Append (Utilities|String|Append ":" (Utilities|String|ToString(Integer) (Math|Float|Round (/ (Math|Vector|VectorLength (- (Transformation|GetActorLocation (Game|Player|GetPlayerPawn 0)) (Transformation|GetActorLocation _array_element))) 1e+02)))) "m")))
    (if (> (Math|Vector|DotProduct (Math|Vector|GetForwardVector (Pawn|GetControlRotation (Game|Player|GetPlayerPawn 0) :!class /Script/Engine.Pawn)) (Math|Vector|Normalize (- (Transformation|GetActorLocation (Game|Player|GetPlayerPawn 0)) (Transformation|GetActorLocation _array_element)))) 0.0)
      (if (> (Math|Vector|DotProduct (Transformation|GetActorForwardVector (Game|Player|GetPlayerPawn 0)) (- (Transformation|GetActorLocation (Game|Player|GetPlayerPawn 0)) (Transformation|GetActorLocation _array_element))) 0.0) :!label _label
        (if (<= (- (.Y (Math|Vector2D|BreakVector2D (Math|Conversions|ToVector2D(Vector) (Class|HUD|Project (Transformation|GetActorLocation _array_element))))) (/ (.y (Viewport|GetViewportSize)) 2.0)) 0.0)
          (Canvas|DrawMaterial 0 (+ (* (Math|Trig|Cos(Degrees) (Class|KismetMathLibrary|DegAcos (* (.x (Math|Vector2D|Normalize2D (- (/ (Viewport|GetViewportSize) 2.0) (Math|Conversions|ToVector2D(Vector) (Class|HUD|Project (Transformation|GetActorLocation _array_element)))))) -1.0))) 1.0 (Variables|Default|GetCircle%20Radius)) (.x _returnvalue_6)) (Math|Float|Clamp(Float) (+ (* (Math|Trig|Sin(Degrees) (Class|KismetMathLibrary|DegAcos (* (.x (Math|Vector2D|Normalize2D (- (/ (Viewport|GetViewportSize) 2.0) (Math|Conversions|ToVector2D(Vector) (Class|HUD|Project (Transformation|GetActorLocation _array_element)))))) -1.0))) 1.0 (Variables|Default|GetCircle%20Radius)) (.y _returnvalue_6)) 5e+01 (- (.y (Viewport|GetViewportSize)) 5e+01)) 128.0 128.0 1024.0 1024.0 1.0 1.0 0.2 false (* (- (Class|KismetMathLibrary|DegAcos (* (.x (Math|Vector2D|Normalize2D (- (/ (Viewport|GetViewportSize) 2.0) (Math|Conversions|ToVector2D(Vector) (Class|HUD|Project (Transformation|GetActorLocation _array_element)))))) -1.0)) 2.7e+02) -1.0) "(X=0.500000,Y=0.500000)")
          (HUD|DrawText (Variables|Default|GetObjective%20Text) "(R=1.000000,G=1.000000,B=1.000000,A=1.000000)" (+ (+ (* (Math|Trig|Cos(Degrees) (Class|KismetMathLibrary|DegAcos (* (.x (Math|Vector2D|Normalize2D (- (/ (Viewport|GetViewportSize) 2.0) (Math|Conversions|ToVector2D(Vector) (Class|HUD|Project (Transformation|GetActorLocation _array_element)))))) -1.0))) 1.0 (Variables|Default|GetCircle%20Radius)) (.x _returnvalue_6)) (Variables|Default|GetX%20Position%20Text%20Buffer)) (+ (Math|Float|Clamp(Float) (+ (* (Math|Trig|Sin(Degrees) (Class|KismetMathLibrary|DegAcos (* (.x (Math|Vector2D|Normalize2D (- (/ (Viewport|GetViewportSize) 2.0) (Math|Conversions|ToVector2D(Vector) (Class|HUD|Project (Transformation|GetActorLocation _array_element)))))) -1.0))) 1.0 (Variables|Default|GetCircle%20Radius)) (.y _returnvalue_6)) 5e+01 (- (.y (Viewport|GetViewportSize)) 5e+01)) (Variables|Default|GetY%20Position%20Text%20Buffer)) "/Engine/EngineFonts/RobotoDistanceField.RobotoDistanceField" 0.5 false)
          (else
            (Canvas|DrawMaterial 0 (+ (* (Math|Trig|Cos(Degrees) (Class|KismetMathLibrary|DegAcos (* (.x (Math|Vector2D|Normalize2D (- (/ (Viewport|GetViewportSize) 2.0) (Math|Conversions|ToVector2D(Vector) (Class|HUD|Project (Transformation|GetActorLocation _array_element)))))) -1.0))) 1.0 (Variables|Default|GetCircle%20Radius)) (.x _returnvalue_5)) (Math|Float|Clamp(Float) (+ (* (Math|Trig|Sin(Degrees) (Class|KismetMathLibrary|DegAcos (* (.x (Math|Vector2D|Normalize2D (- (/ (Viewport|GetViewportSize) 2.0) (Math|Conversions|ToVector2D(Vector) (Class|HUD|Project (Transformation|GetActorLocation _array_element)))))) -1.0))) -1.0 (Variables|Default|GetCircle%20Radius)) (.y _returnvalue_5)) 5e+01 (- (.y (Viewport|GetViewportSize)) 5e+01)) 128.0 128.0 1024.0 1024.0 1.0 1.0 0.2 false (- (Class|KismetMathLibrary|DegAcos (* (.x (Math|Vector2D|Normalize2D (- (/ (Viewport|GetViewportSize) 2.0) (Math|Conversions|ToVector2D(Vector) (Class|HUD|Project (Transformation|GetActorLocation _array_element)))))) -1.0)) 9e+01) "(X=0.500000,Y=0.500000)")
            (HUD|DrawText (Variables|Default|GetObjective%20Text) "(R=1.000000,G=1.000000,B=1.000000,A=1.000000)" (+ (+ (* (Math|Trig|Sin(Degrees) (Class|KismetMathLibrary|DegAcos (* (.x (Math|Vector2D|Normalize2D (- (/ (Viewport|GetViewportSize) 2.0) (Math|Conversions|ToVector2D(Vector) (Class|HUD|Project (Transformation|GetActorLocation _array_element)))))) -1.0))) -1.0 (Variables|Default|GetCircle%20Radius)) (.y _returnvalue_5)) (Variables|Default|GetX%20Position%20Text%20Buffer)) (+ (Math|Float|Clamp(Float) (+ (* (Math|Trig|Sin(Degrees) (Class|KismetMathLibrary|DegAcos (* (.x (Math|Vector2D|Normalize2D (- (/ (Viewport|GetViewportSize) 2.0) (Math|Conversions|ToVector2D(Vector) (Class|HUD|Project (Transformation|GetActorLocation _array_element)))))) -1.0))) -1.0 (Variables|Default|GetCircle%20Radius)) (.y _returnvalue_5)) 5e+01 (- (.y (Viewport|GetViewportSize)) 5e+01)) (Variables|Default|GetY%20Position%20Text%20Buffer)) "/Engine/EngineFonts/RobotoDistanceField.RobotoDistanceField" 0.5 false)))
        (elif (<= (- (.Y (Math|Vector2D|BreakVector2D (Math|Conversions|ToVector2D(Vector) (Class|HUD|Project (Transformation|GetActorLocation _array_element))))) (/ (.y (Viewport|GetViewportSize)) 2.0)) 0.0)
          (Canvas|DrawMaterial 0 (+ (* (Math|Trig|Cos(Degrees) (* (Class|KismetMathLibrary|DegAcos (* (.x (Math|Vector2D|Normalize2D (- (/ (Viewport|GetViewportSize) 2.0) (Math|Conversions|ToVector2D(Vector) (Class|HUD|Project (Transformation|GetActorLocation _array_element)))))) -1.0)) -1.0)) (Variables|Default|GetCircle%20Radius)) (.x _returnvalue_8)) (Math|Float|Clamp(Float) (+ (* (Math|Trig|Sin(Degrees) (* (Class|KismetMathLibrary|DegAcos (* (.x (Math|Vector2D|Normalize2D (- (/ (Viewport|GetViewportSize) 2.0) (Math|Conversions|ToVector2D(Vector) (Class|HUD|Project (Transformation|GetActorLocation _array_element)))))) -1.0)) -1.0)) (Variables|Default|GetCircle%20Radius)) (.y _returnvalue_8)) 5e+01 (- (.y (Viewport|GetViewportSize)) 5e+01)) 128.0 128.0 1024.0 1024.0 1.0 1.0 0.2 false (* (- (Class|KismetMathLibrary|DegAcos (* (.x (Math|Vector2D|Normalize2D (- (/ (Viewport|GetViewportSize) 2.0) (Math|Conversions|ToVector2D(Vector) (Class|HUD|Project (Transformation|GetActorLocation _array_element)))))) -1.0)) 9e+01) -1.0) "(X=0.500000,Y=0.500000)")
          (HUD|DrawText (Variables|Default|GetObjective%20Text) "(R=1.000000,G=1.000000,B=1.000000,A=1.000000)" (+ (+ (* (Math|Trig|Cos(Degrees) (* (Class|KismetMathLibrary|DegAcos (* (.x (Math|Vector2D|Normalize2D (- (/ (Viewport|GetViewportSize) 2.0) (Math|Conversions|ToVector2D(Vector) (Class|HUD|Project (Transformation|GetActorLocation _array_element)))))) -1.0)) -1.0)) (Variables|Default|GetCircle%20Radius)) (.x _returnvalue_8)) (Variables|Default|GetX%20Position%20Text%20Buffer)) (+ (Math|Float|Clamp(Float) (+ (* (Math|Trig|Sin(Degrees) (* (Class|KismetMathLibrary|DegAcos (* (.x (Math|Vector2D|Normalize2D (- (/ (Viewport|GetViewportSize) 2.0) (Math|Conversions|ToVector2D(Vector) (Class|HUD|Project (Transformation|GetActorLocation _array_element)))))) -1.0)) -1.0)) (Variables|Default|GetCircle%20Radius)) (.y _returnvalue_8)) 5e+01 (- (.y (Viewport|GetViewportSize)) 5e+01)) (Variables|Default|GetY%20Position%20Text%20Buffer)) "/Engine/EngineFonts/RobotoDistanceField.RobotoDistanceField" 0.5 false)
          (else
            (Canvas|DrawMaterial 0 (+ (* (Math|Trig|Cos(Degrees) (Class|KismetMathLibrary|DegAcos (* (.x (Math|Vector2D|Normalize2D (- (/ (Viewport|GetViewportSize) 2.0) (Math|Conversions|ToVector2D(Vector) (Class|HUD|Project (Transformation|GetActorLocation _array_element)))))) 1.0))) 1.0 (Variables|Default|GetCircle%20Radius)) (.x _returnvalue_7)) (Math|Float|Clamp(Float) (+ (* (Math|Trig|Sin(Degrees) (Class|KismetMathLibrary|DegAcos (* (.x (Math|Vector2D|Normalize2D (- (/ (Viewport|GetViewportSize) 2.0) (Math|Conversions|ToVector2D(Vector) (Class|HUD|Project (Transformation|GetActorLocation _array_element)))))) 1.0))) 1.0 (Variables|Default|GetCircle%20Radius)) (.y _returnvalue_7)) 5e+01 (- (.y (Viewport|GetViewportSize)) 5e+01)) 128.0 128.0 1024.0 1024.0 1.0 1.0 0.2 false (- (Class|KismetMathLibrary|DegAcos (* (.x (Math|Vector2D|Normalize2D (- (/ (Viewport|GetViewportSize) 2.0) (Math|Conversions|ToVector2D(Vector) (Class|HUD|Project (Transformation|GetActorLocation _array_element)))))) 1.0)) 2.7e+02) "(X=0.500000,Y=0.500000)")
            (HUD|DrawText (Variables|Default|GetObjective%20Text) "(R=1.000000,G=1.000000,B=1.000000,A=1.000000)" (+ (+ (* (Math|Trig|Cos(Degrees) (Class|KismetMathLibrary|DegAcos (* (.x (Math|Vector2D|Normalize2D (- (/ (Viewport|GetViewportSize) 2.0) (Math|Conversions|ToVector2D(Vector) (Class|HUD|Project (Transformation|GetActorLocation _array_element)))))) 1.0))) 1.0 (Variables|Default|GetCircle%20Radius)) (.x _returnvalue_7)) (Variables|Default|GetX%20Position%20Text%20Buffer)) (+ (Math|Float|Clamp(Float) (+ (* (Math|Trig|Sin(Degrees) (Class|KismetMathLibrary|DegAcos (* (.x (Math|Vector2D|Normalize2D (- (/ (Viewport|GetViewportSize) 2.0) (Math|Conversions|ToVector2D(Vector) (Class|HUD|Project (Transformation|GetActorLocation _array_element)))))) 1.0))) 1.0 (Variables|Default|GetCircle%20Radius)) (.y _returnvalue_7)) 5e+01 (- (.y (Viewport|GetViewportSize)) 5e+01)) (Variables|Default|GetY%20Position%20Text%20Buffer)) "/Engine/EngineFonts/RobotoDistanceField.RobotoDistanceField" 0.5 false))))
      (elif (<= (Math|Vector|DotProduct (Math|Vector|GetForwardVector (Pawn|GetControlRotation (Game|Player|GetPlayerPawn 0) :!class /Script/Engine.Pawn)) (Math|Vector|Normalize (- (Transformation|GetActorLocation (Game|Player|GetPlayerPawn 0)) (Transformation|GetActorLocation _array_element)))) 0.66)
        (if (and (> (.y (.ScreenPosition (Class|WidgetLayoutLibrary|ProjectWorldLocationtoWidgetPosition (Game|GetPlayerController 0) (Transformation|GetActorLocation _array_element)))) 0.0) (<= (.y (.ScreenPosition (Class|WidgetLayoutLibrary|ProjectWorldLocationtoWidgetPosition (Game|GetPlayerController 0) (Transformation|GetActorLocation _array_element)))) (+ (.y (Viewport|GetViewportSize)) (Variables|Default|GetY%20Position%20Buffer))))
          (if (> (.Z (Math|Vector|BreakVector (Class|HUD|Project (Transformation|GetActorLocation _array_element)))) 0.0)
            (HUD|DrawText (Variables|Default|GetObjective%20Text) "(R=1.000000,G=1.000000,B=1.000000,A=1.000000)" (+ (- (.X (Math|Vector|BreakVector (Class|HUD|Project (Transformation|GetActorLocation _array_element)))) (/ (.OutWidth (Class|HUD|GetTextSize (Utilities|String|Append "Objective" (Utilities|String|Append (Utilities|String|Append ":" (Utilities|String|ToString(Integer) (Math|Float|Round (/ (Math|Vector|VectorLength (- (Transformation|GetActorLocation (Game|Player|GetPlayerPawn 0)) (Transformation|GetActorLocation _array_element))) 1e+02)))) "m")) "/Engine/EngineFonts/RobotoDistanceField.RobotoDistanceField" 1.0)) 2.0)) 3e+01) (- (.Y (Math|Vector|BreakVector (Class|HUD|Project (Transformation|GetActorLocation _array_element)))) 1e+02) "/Engine/EngineFonts/RobotoDistanceField.RobotoDistanceField" 0.5 false)
            (Class|HUD|DrawMaterialSimple 0 (+ (- (.X (Math|Vector|BreakVector (Class|HUD|Project (Transformation|GetActorLocation _array_element)))) (/ (.OutWidth (Class|HUD|GetTextSize (Utilities|String|Append "Objective" (Utilities|String|Append (Utilities|String|Append ":" (Utilities|String|ToString(Integer) (Math|Float|Round (/ (Math|Vector|VectorLength (- (Transformation|GetActorLocation (Game|Player|GetPlayerPawn 0)) (Transformation|GetActorLocation _array_element))) 1e+02)))) "m")) "/Engine/EngineFonts/RobotoDistanceField.RobotoDistanceField" 1.0)) 2.0)) 5e+01) (- (.Y (Math|Vector|BreakVector (Class|HUD|Project (Transformation|GetActorLocation _array_element)))) 85.0) 256.0 256.0 1.0 false))
          (else
            (goto _label)))
        (else
          (goto _label))))))

(fn ConstructionScript)