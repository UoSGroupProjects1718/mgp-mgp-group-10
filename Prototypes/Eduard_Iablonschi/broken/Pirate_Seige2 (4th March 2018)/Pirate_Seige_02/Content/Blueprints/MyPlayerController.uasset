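; Player controller that lets the player cycle possession between the 2D side-scroller characters in the level.
; On BeginPlay it caches every such character in an array and possesses the one at the current index.
; Left-click steps a looping MultiGate whose Out 1 possesses the next character, wrapping at the end; other outputs do nothing.
; An unfinished bullet spawn and follow-camera chain is left disconnected, with no class set.
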(event EventBeginPlay
  ;[1 1 1] Stores all actors of one class in an array (2DSide Scroller Character)
  (bind _outactors (Actor|GetAllActorsOfClass "/Game/2DSideScrollerBP/Blueprints/2DSideScrollerCharacter.2DSideScrollerCharacter_C"))
  (bind _output_get (Variables|Default|SetAvailableCharacters _outactors))
  (Pawn|Possess (Utilities|Array|Get(acopy) _output_get (Variables|Default|GetCurrentSelectedCharacterIndex))))

(event Input|MouseEvents|LeftMouseButton
  (params (Key :type Key%20Structure))
  ;[1 1 1] If LMB is pressed, 3 actions : shoot, change player, and (to be added)
  (:Pressed
    (Utilities|FlowControl|MultiGate false true -1
      (:Out%201
        (if (>= (Variables|Default|GetCurrentSelectedCharacterIndex) (- (Utilities|Array|Length (Variables|Default|GetAvailableCharacters)) 1))
          (Variables|Default|SetCurrentSelectedCharacterIndex 0)
          (else
            (Variables|Default|SetCurrentSelectedCharacterIndex (+ (Variables|Default|GetCurrentSelectedCharacterIndex) 1))))
        (Pawn|Possess (Utilities|Array|Get(acopy) (Variables|Default|GetAvailableCharacters) (Variables|Default|GetCurrentSelectedCharacterIndex)))))))

(fn ConstructionScript)